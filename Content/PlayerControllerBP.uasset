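; Player controller Blueprint that sets up the local player's HUD and provides a manual save hotkey.
; When play begins on a local controller, it creates the Main_HUD widget, adds it to the viewport and switches input to game-only.
; Pressing L casts the game mode to GameModeBP, calls its WriteSaveGame and prints a green "GAME SAVED" message.
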(event EventBlueprintBeginPlayingState
  (if (Pawn|IsLocalController)
    (bind _returnvalue (UserInterface|CreateWidget "/Game/Context/UI/Main_HUD.Main_HUD_C"))
    (UserInterface|Viewport|AddtoViewport _returnvalue 0)
    (Input|SetInputModeGameOnly self)))

(event Input|KeyboardEvents|L
  (params (Key :type Key%20Structure :default "None"))
  (:Pressed
    (bind _asgame_mode_bp (Utilities|Casting|CastToGameModeBP (Game|GetGameMode)))
    (Class|ActionGameModeBase|WriteSaveGame _asgame_mode_bp)
    (Development|PrintString "GAME SAVED" true true "(R=0.061988,G=1.000000,B=0.156656,A=1.000000)")))

(fn ConstructionScript)