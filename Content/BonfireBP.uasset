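; Interactable bonfire actor that lights its fire and saves the game when used.
; Interaction sets the FireActivate flag, has GameModeBP write the save game, prints a confirmation, then activates the particle system through UpdateFlames.
; OnActorLoaded also calls UpdateFlames, so the flames turn on at load if the flag is set.
; Its interact text is empty.
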(event Custom|UpdateFlames
  (if (Variables|Default|GetbFireActivate)
    (Components|Activation|Activate (Variables|Default|GetParticleSystem) false)))

(event EventInteraction
  (params (InstigatorPawn :type Pawn%20Object%20Reference))
  (Variables|Default|SetbFireActivate true)
  (bind _asgame_mode_bp (Utilities|Casting|CastToGameModeBP (Game|GetGameMode)))
  (Class|ActionGameModeBase|WriteSaveGame _asgame_mode_bp)
  (Development|PrintString "WORLD_Saved" true true "(R=0.165414,G=1.000000,B=0.262566,A=1.000000)")
  (CallFunction|UpdateFlames))

(event EventOnActorLoaded
  (CallFunction|UpdateFlames))

(fn ConstructionScript)

(fn GetInteractText
  (params (InstigatorPawn :type Pawn%20Object%20Reference))
  (return ""))