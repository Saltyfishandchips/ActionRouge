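; Main player character Blueprint that handles parry input and spawns an attached health widget.
; Pressing Parry starts the "Parry" action by name through the action component.
; BeginPlay creates a MinionHP_Widget with the character as its attached actor and adds it to the viewport.
; An unconnected delayed chain that would apply Effect_Stunned never runs, and the construction script is empty.
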(event EventBeginPlay
  (bind _returnvalue (UserInterface|CreateWidget "/Game/Context/UI/MinionHP_Widget.MinionHP_Widget_C" 0 self))
  (UserInterface|Viewport|AddtoViewport _returnvalue 0))

(event Input|ActionEvents|InputActionParry
  (params (Key :type Key%20Structure :default "None"))
  (:Pressed
    (Class|ActionComponent|StartActionbyName (Variables|Default|GetActionComp) self "Parry")))

(fn ConstructionScript)